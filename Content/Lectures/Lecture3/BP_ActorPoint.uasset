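; BP_ActorPoint is a pickup that adds its Points value, positive or negative, to the first-person character's score.
; On BeginPlay it colors its mesh green for non-negative values or red for negative ones, then caches the player character.
; When that player overlaps it while their PlayerPoints is below a fixed cap, it applies the value, prints the new total and destroys itself.
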(event `self.ReceiveBeginPlay`
  (bind _staticmesh (`self.StaticMesh`))
  (if (>= (`self.Points`) 0)
    (`PrimitiveComponent.SetMaterial` _staticmesh 0 "/Game/Lectures/Lecture3/GreenM.GreenM")
    (else
      (`PrimitiveComponent.SetMaterial` _staticmesh 0 "/Game/Lectures/Lecture3/RedM.RedM")))
  (bind _asbp_first_person_character (cast `/Game/FirstPerson/Blueprints/BP_FirstPersonCharacter` (`GameplayStatics.GetPlayerCharacter` 0)))
  (set `self.As BP First Person Character` _asbp_first_person_character))

(event `self.ReceiveActorBeginOverlap`
  (params (OtherActor :type "Actor Object Reference"))
  (bind _playerpoints (`/Game/FirstPerson/Blueprints/BP_FirstPersonCharacter.PlayerPoints` (`self.As BP First Person Character`)))
  (if (and (== OtherActor (`self.As BP First Person Character`)) (> 50 _playerpoints))
    (bind _output_get (set `/Game/FirstPerson/Blueprints/BP_FirstPersonCharacter.PlayerPoints` (+ _playerpoints (`self.Points`)) (`self.As BP First Person Character`)))
    (`KismetSystemLibrary.PrintString` (`KismetStringLibrary.Conv_IntToString` _output_get))
    (`self.K2_DestroyActor`)))

(fn `UserConstructionScript`)