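; BP_ActorPassword is a pickup that displays its Key as text and adds it to the player's password.
; On BeginPlay it sets the TextRender from Key and caches the player's BP_FirstPersonCharacter.
; When that character overlaps it, the actor appends Key to the character's Password string and destroys itself.
; Every Tick it rotates the text to face the player camera.
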(event `self.ReceiveBeginPlay`
  (`TextRenderComponent.K2_SetText` (`self.TextRender`) (`KismetTextLibrary.Conv_StringToText` (`self.Key`)))
  (bind _asbp_first_person_character (cast `/Game/FirstPerson/Blueprints/BP_FirstPersonCharacter` (`GameplayStatics.GetPlayerCharacter` 0)))
  (set `self.As BP First Person Character` _asbp_first_person_character))

(event `self.ReceiveActorBeginOverlap`
  (params (OtherActor :type "Actor Object Reference"))
  (bind _as_bp_first_person_character (`self.As BP First Person Character`))
  (if (== OtherActor (`self.As BP First Person Character`))
    (set `/Game/FirstPerson/Blueprints/BP_FirstPersonCharacter.Password` (`KismetStringLibrary.Concat_StrStr` (`/Game/FirstPerson/Blueprints/BP_FirstPersonCharacter.Password` _as_bp_first_person_character) (`self.Key`)) _as_bp_first_person_character)
    (`self.K2_DestroyActor`)))

(event `self.ReceiveTick`
  (params (DeltaSeconds :type "Float (single-precision)"))
  (`SceneComponent.K2_SetWorldRotation` (`self.TextRender`) (`KismetMathLibrary.FindLookAtRotation` (`self.K2_GetActorLocation`) (`PlayerCameraManager.GetCameraLocation` (`GameplayStatics.GetPlayerCameraManager` 0))) false false))

(fn `UserConstructionScript`)